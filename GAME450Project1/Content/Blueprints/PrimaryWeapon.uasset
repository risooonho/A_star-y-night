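; PrimaryWeapon is a weapon Blueprint that fires a PrimaryProjectile while it has loaded ammo.
; Its Fire event checks LoadedAmmo, waits briefly, then spawns the projectile slightly ahead of the Tip component, offset and rotated along the player character's camera.
; A scaled-down explosion emitter at the tip serves as muzzle flash, and each shot decrements LoadedAmmo.
; It handles no reloading, and the construction script is empty.
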(event `Fire`
  (if (not (== (`self.LoadedAmmo`) 0))
    (bind _asue_4asp_character (cast `/Game/AnimStarterPack/Ue4ASP_Character` (`GameplayStatics.GetPlayerCharacter` 0)))
    (`KismetSystemLibrary.Delay` 0.1)
    (bind _returnvalue (`SceneComponent.K2_GetComponentRotation` (`/Game/AnimStarterPack/Ue4ASP_Character.PlayerCamera` _asue_4asp_character)))
    (`|SpawnActorFromClass` "/Game/Blueprints/PrimaryProjectile.PrimaryProjectile_C" (`KismetMathLibrary.MakeTransform` (+ (`SceneComponent.K2_GetComponentLocation` (`self.Tip`)) (`KismetMathLibrary.GreaterGreater_VectorRotator` (100.0 0.0 0.0) _returnvalue)) _returnvalue) "Undefined" "OverrideRootScale" null null)
    (`GameplayStatics.SpawnEmitterAtLocation` "/Game/StarterContent/Particles/P_Explosion.P_Explosion" (`SceneComponent.K2_GetComponentLocation` (`self.Tip`)) (struct) (0.05 0.05 0.05))
    (set `self.LoadedAmmo` (- (`self.LoadedAmmo`) 1))))

(fn `UserConstructionScript`)