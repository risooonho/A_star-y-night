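; HeavyProjectile is an explosive projectile that damages zombie AI and detonates on hit.
; If the hit actor is a ZombieAI, it subtracts Damage directly from that zombie's Health.
; A DoOnce then fires the ExplosiveForce impulse, spawns an enlarged explosion emitter at that component's location, and destroys the projectile.
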(event `self.ReceiveHit`
  (params (MyComp :type "PrimitiveComponent Object Reference") (Other :type "Actor Object Reference") (OtherComp :type "PrimitiveComponent Object Reference") (bSelfMoved :type Boolean) (HitLocation :type "Vector Structure") (HitNormal :type "Vector Structure") (NormalImpulse :type "Vector Structure") (Hit :type "HitResult Structure (by ref)"))
  (bind _explosiveforce (`self.ExplosiveForce`))
  (bind _aszombie_ai (cast `/Game/Blueprints/ZombieAI` Other)
    (:`then`
      (set `/Game/Blueprints/ZombieAI.Health` (- (`/Game/Blueprints/ZombieAI.Health` _aszombie_ai) (`self.Damage`)) _aszombie_ai))
    (:`CastFailed`
      _))
  (`/Engine/EditorBlueprintResources/StandardMacros.DoOnce` false
    (:`Completed`
      (`RadialForceComponent.FireImpulse` _explosiveforce)
      (`GameplayStatics.SpawnEmitterAtLocation` "/Game/StarterContent/Particles/P_Explosion.P_Explosion" (`SceneComponent.K2_GetComponentLocation` _explosiveforce) (struct) (3.0 3.0 3.0))
      (`self.K2_DestroyActor`))))

(fn `UserConstructionScript`)