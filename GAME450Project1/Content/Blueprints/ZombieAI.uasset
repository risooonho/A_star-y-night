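; Zombie enemy that rises from its spawn point in a smoke effect, then chases the player character.
; A Spawn timeline drives the rise and starts an AI MoveTo when finished, while PawnSensing sight and noise events reissue moves toward detected player characters.
; On hit, zero health triggers a ragdoll death and delayed destruction; otherwise it calls DamageCharacter on player characters, which is still an empty stub.
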(event `self.ReceiveBeginPlay`
  (set `self.InitialLoc` (`self.K2_GetActorLocation`))
  (bind _asue_4asp_character (cast `/Game/AnimStarterPack/Ue4ASP_Character` (`GameplayStatics.GetPlayerCharacter` 0)))
  (`GameplayStatics.SpawnEmitterAtLocation` "/Game/AdvancedVillagePack/Effects/Pfx_SmokeChimney.Pfx_SmokeChimney" (+ (`self.InitialLoc`) (0.0 0.0 100.0)) (struct) (3.0 3.0 3.0))
  (bind (_direction _rise) (`Timeline|Spawn` :!via `PlayFromStart`)
    (:`Update`
      (`self.K2_SetActorLocation` (+ _rise (`self.InitialLoc`))))
    (:`Finished`
      (`AITask_MoveTo.AIMoveTo` (`AIBlueprintHelperLibrary.GetAIController` self) (`self.K2_GetActorLocation` _asue_4asp_character) _asue_4asp_character))))

(event `self.ReceiveHit`
  (params (MyComp :type "PrimitiveComponent Object Reference") (Other :type "Actor Object Reference") (OtherComp :type "PrimitiveComponent Object Reference") (bSelfMoved :type Boolean) (HitLocation :type "Vector Structure") (HitNormal :type "Vector Structure") (NormalImpulse :type "Vector Structure") (Hit :type "HitResult Structure (by ref)"))
  (if (<= (`self.Health`) 0)
    (`self.Death`)
    (`KismetSystemLibrary.Delay` 5.0)
    (`self.K2_DestroyActor`)
    (else
      (bind _asue_4asp_character (cast `/Game/AnimStarterPack/Ue4ASP_Character` Other))
      (`self.DamageCharacter` _asue_4asp_character))))

(event `self.PawnSensing.OnSeePawn`
  (params (Pawn :type "Pawn Object Reference"))
  (bind _asue_4asp_character (cast `/Game/AnimStarterPack/Ue4ASP_Character` Pawn))
  (`|AIMoveTo` self (`self.K2_GetActorLocation` _asue_4asp_character) _asue_4asp_character))

(event `self.PawnSensing.OnHearNoise`
  (params (Instigator :type "Pawn Object Reference") (Location :type "Vector Structure (by ref)") (Volume :type "Float (single-precision)"))
  (bind _asue_4asp_character (cast `/Game/AnimStarterPack/Ue4ASP_Character` Instigator))
  (`|AIMoveTo` self (`self.K2_GetActorLocation` _asue_4asp_character) _asue_4asp_character))

(fn `DamageCharacter`
  (params (Character :type "/Game/AnimStarterPack/Ue4ASP_Character Object Reference")))

(fn `Death`
  (`PrimitiveComponent.SetSimulatePhysics` (`self.Mesh`) true)
  (set `self.IsDead` true))

(fn `UserConstructionScript`)