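; A zombie game mode that spawns a ZombieAI enemy when play begins.
; On BeginPlay it gathers all ZombieSpawnPoint actors, waits briefly, then calls its Spawn event once.
; Spawn places the zombie at a randomly chosen point's transform and always spawns it, ignoring collisions.
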(event `self.ReceiveBeginPlay`
  (bind _outactors (`GameplayStatics.GetAllActorsOfClass` "/Game/Blueprints/ZombieSpawnPoint.ZombieSpawnPoint_C"))
  (set `self.SpawnPoints` _outactors)
  (`KismetSystemLibrary.Delay` 0.2)
  (`self.Spawn`))

(event `Spawn`
  (bind _spawnpoints (`self.SpawnPoints`))
  (`|SpawnActorFromClass` "/Game/Blueprints/ZombieAI.ZombieAI_C" (`self.GetTransform` (`|GetArrayItem` _spawnpoints (`KismetMathLibrary.RandomIntegerInRange` 0 (- (`KismetArrayLibrary.Array_Length` _spawnpoints) 1)))) "AlwaysSpawn" "OverrideRootScale" null null))

(fn `UserConstructionScript`)